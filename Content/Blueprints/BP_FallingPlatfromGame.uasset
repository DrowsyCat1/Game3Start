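; A falling platform that drops away when the player character steps on it.
; On the first overlap of its Box by the third-person character, the Cube turns red and starts simulating physics, then the actor destroys itself after a short delay.
; A reset path with a green material and a timeline lerp back to the saved start transform is present but disconnected, so the platform never returns.
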(event OnComponentBeginOverlap(Box)
  (params (OverlappedComponent :type Primitive%20Component%20Object%20Reference) (OtherActor :type Actor%20Object%20Reference) (OtherComp :type Primitive%20Component%20Object%20Reference) (OtherBodyIndex :type Integer) (bFromSweep :type Boolean) (SweepResult :type Hit%20Result%20Structure%20%28by%20ref%29))
  (Utilities|Casting|CastToBP_ThirdPersonCharacter OtherActor) ; Is it the player that is standing on us?
  (if (not (Variables|Default|GetActive)) ; are we doing things?
    (Variables|Default|SetActive true) ; No? Well let's do things now!
    (Rendering|Material|SetMaterial (Variables|Default|GetCube) 0 "/AnimationSharing/AnimSharingRed.AnimSharingRed") ; Turning red beacuse we're falling now.
    (Physics|SetSimulatePhysics (Variables|Default|GetCube) true)
    (Utilities|FlowControl|Delay 0.8)
    (Actor|DestroyActor)))

(event EventBeginPlay
  (Variables|Default|SetStarting%20Transform (Transformation|GetWorldTransform (Variables|Default|GetCube)))
  (Variables|Default|SetStartingMaterial (Rendering|Material|GetMaterial (Variables|Default|GetCube) 0)))

(fn ConstructionScript)