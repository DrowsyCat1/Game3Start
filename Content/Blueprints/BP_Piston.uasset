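; BP_Piston is an animated piston that moves up and down with sound, vibration and camera shake.
; On BeginPlay it starts a Timeline with a random float, whose track drives the Piston component's relative Z position.
; The Timeline's Thud event spawns a quiet, low-pitched sound with random variation, plays force feedback and starts a source-based camera shake on player 0.
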(event EventBeginPlay
  (Utilities|FlowControl|Sequence
    (:then_0
      (bind _newtrack_0 (Timeline|Timeline Play)
        (:Update
          (Transformation|SetRelativeLocation (Variables|Default|GetPiston) (Math|Vector|MakeVector 0.0 0.0 (- (* _newtrack_0 4e+01) 2e+01)) false false))
        (:Thud
          (Audio|SpawnSoundatLocation "/Game/Audio/HitHurt5OneShot.HitHurt5OneShot" (Transformation|GetWorldLocation (Variables|Default|GetPiston)) "0, 0, 0" (Math|Random|RandomFloatinRange 0.0 0.3) (Math|Random|RandomFloatinRange 0.01 0.2) 0.0 0 0)
          (Audio|Components|Audio|Play (Variables|Default|GetForceFeedback) 0.0)
          (Class|PlayerController|ClientStartCameraShakefromSource (Game|GetPlayerController 0) 0 (Variables|Default|GetSource%20Component)))))
    (:then_1
      (Timeline|Timeline SetNewTime))))

(event Collision|EventActorBeginOverlap
  (params (OtherActor :type Actor%20Object%20Reference)))

(event EventTick
  (params (DeltaSeconds :type Float%20%28single-precision%29)))

(fn ConstructionScript)